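; Racing game mode that runs a timed checkpoint race from start menu through countdown to win or lose screen.
; The selected difficulty sets a multiplier for time awarded by checkpoints, and the countdown's end unlocks driving and starts the timer.
; Checkpoints extend time by re-setting the timer with remaining plus bonus time, playing a HUD animation.
; Finish line or timeout feeds a guarded GameEnd, whose widget can reload the level.
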(event `self.ReceiveBeginPlay`
  (`|ExecutionSequence`
    (:`then_0`
      (bind _returnvalue (`|CreateWidget` "/Game/RacingGame/Widgets/W_StartMenu.W_StartMenu_C"))
      (bind _output_get (set `self.W_StartMenu` _returnvalue))
      (`UserWidget.AddToViewport` _output_get 0))
    (:`then_1`
      (bind _outactors (`GameplayStatics.GetAllActorsOfClass` "/Game/RacingGame/Checkpoints/BP_Checkpoint.BP_Checkpoint_C"))
      (for _array_element _outactors
        (if (`/Game/RacingGame/Checkpoints/BP_Checkpoint.IsFinishLine` _array_element)
          (add `/Game/RacingGame/Checkpoints/BP_Checkpoint.OnCheckpointCrossed` _array_element (`|CreateDelegate` :!event `Win_CrossTheFinishLine`))
          (else
            (add `/Game/RacingGame/Checkpoints/BP_Checkpoint.OnCheckpointCrossedWithTime` _array_element (`|CreateDelegate` :!event `CrossedCheckpoint`))))))
    (:`then_2`
      (add `/Game/RacingGame/Widgets/W_StartMenu.DifficultySelected` (`self.W_StartMenu`) (delegate `DifficultySelected`)))))

(event `DifficultySelected`
  (params (TimeMultiplier :type "Float (double-precision)"))
  (set `self.CheckPointTimeMultiplier` TimeMultiplier)
  (`self.Start Countdown`))

(event `Start Countdown`
  (`KismetSystemLibrary.PrintString` "Start Countdown ")
  (bind _returnvalue (`|CreateWidget` "/Game/RacingGame/Widgets/W_CountDown.W_CountDown_C" null (`KismetMathLibrary.FTrunc` (`self.StartCountdownDuration`))))
  (`UserWidget.AddToViewport` _returnvalue 0)
  (add `/Game/RacingGame/Widgets/W_CountDown.CountDownEnded` _returnvalue (delegate `Game Start`)))

(event `Game Start`
  (set `self.GameEnded` false)
  (bind _returnvalue (`GameplayStatics.GetActorOfClass` "/Game/VehicleTemplate/Blueprints/VehicleAdvPawn.VehicleAdvPawn_C"))
  (set `/Game/VehicleTemplate/Blueprints/VehicleAdvPawn.IsDrivePossible` true _returnvalue)
  (`KismetSystemLibrary.PrintString` "Game has started ")
  (bind _returnvalue_2 (`KismetSystemLibrary.K2_SetTimerDelegate` (delegate `Lose_OutOfTime`) (`self.Start Timer Duration`)))
  (set `self.RemaingTimeHandler` _returnvalue_2))

(event `Lose_OutOfTime`
  (`self.Game End` false))

(event `Win_CrossTheFinishLine`
  (set `self.WinTime` (`KismetSystemLibrary.K2_GetTimerRemainingTimeHandle` (`self.RemaingTimeHandler`)))
  (`KismetSystemLibrary.K2_ClearAndInvalidateTimerHandle` (`self.RemaingTimeHandler`))
  (`self.Game End` true))

(event `CrossedCheckpoint`
  (params (TimeToAdd :type Integer))
  (`self.AddTimeToTimer` (`KismetMathLibrary.FTrunc` (* TimeToAdd (`self.CheckPointTimeMultiplier`)))))

(event `Game End`
  (params (isWon :type Boolean))
  (if (not (`self.GameEnded`))
    (set `PlayerController.bShowMouseCursor` true (`GameplayStatics.GetPlayerController` 0))
    (set `self.GameEnded` true)
    (bind _returnvalue (`|CreateWidget` "/Game/RacingGame/Widgets/W_GameEnded.W_GameEnded_C" null isWon (`self.WinTime`)))
    (`UserWidget.AddToViewport` _returnvalue 0)
    (add `/Game/RacingGame/Widgets/W_GameEnded.GoBackToMenu` _returnvalue (delegate `GameRestarted`))
    (`KismetSystemLibrary.PrintString` (`KismetMathLibrary.SelectString` "You Won!" "You Lose!" isWon))))

(event `GameRestarted`
  (`GameplayStatics.OpenLevelBySoftObjectPtr` "/Game/VehicleTemplate/Maps/VehicleExampleMap.VehicleExampleMap"))

(fn `AddTimeToTimer`
  (params (Time :type Integer))
  (bind _returnvalue (`KismetSystemLibrary.K2_SetTimerDelegate` (`|CreateDelegate` :!event `Lose_OutOfTime`) (+ Time (`KismetSystemLibrary.K2_GetTimerRemainingTimeHandle` (`self.RemaingTimeHandler`)))))
  (set `self.RemaingTimeHandler` _returnvalue)
  (bind _asvehicle_player_controller (cast `/Game/VehicleTemplate/Blueprints/VehiclePlayerController` (`GameplayStatics.GetPlayerController` 0)))
  (`/Game/VehicleTemplate/Blueprints/VehicleUI.PlayAddedTimeAnim` (`/Game/VehicleTemplate/Blueprints/VehiclePlayerController.VehicleHud` _asvehicle_player_controller)))

(fn `UserConstructionScript`)